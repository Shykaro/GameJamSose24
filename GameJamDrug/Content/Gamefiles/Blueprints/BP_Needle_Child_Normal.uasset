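; BP_Needle_Child_Normal is a needle child Blueprint that changes the player character's insanity when the IA_Needle input fires.
; The handler finds BP_ThirdPersonCharacter by class, adds the Sanity value to its InsanityScore and prints the new score.
; It has no proximity check of its own; BeginPlay, overlap and Tick are disabled stubs, and construction only calls the parent.
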(event Input|EnhancedActionEvents|EnhancedInputActionIA_Needle
  (params (ActionValue :type Boolean) (ElapsedSeconds :type Float%20%28double-precision%29) (TriggeredSeconds :type Float%20%28double-precision%29) (InputAction :type Input%20Action%20Object%20Reference :default "/Game/Gamefiles/Input/Actions/IA_Needle.IA_Needle"))
  (bind _returnvalue (Actor|GetActorOfClass "/Game/Gamefiles/Blueprints/BP_ThirdPersonCharacter.BP_ThirdPersonCharacter_C"))
  (Variables|/Game/Gamefiles/Blueprints/BP_ThirdPersonCharacter.BP_ThirdPersonCharacter_C|SetInsanityScore _returnvalue (+ (Variables|/Game/Gamefiles/Blueprints/BP_ThirdPersonCharacter.BP_ThirdPersonCharacter_C|GetInsanityScore _returnvalue) (Variables|Default|Getsanity)))
  (Development|PrintText (Utilities|Text|ToText(Float) (Variables|/Game/Gamefiles/Blueprints/BP_ThirdPersonCharacter.BP_ThirdPersonCharacter_C|GetInsanityScore _returnvalue) "HalfToEven")))

(event EventBeginPlay
  (|CallParentFunction) ; Dieser Knoten ist deaktiviert und wird nicht aufgerufen.\nZiehe die Pins ab, um die Funktionalität aufzubauen.
)

(event Collision|EventActorBeginOverlap
  (params (OtherActor :type Actor%20Object%20Reference))
  (|CallParentFunction OtherActor) ; Dieser Knoten ist deaktiviert und wird nicht aufgerufen.\nZiehe die Pins ab, um die Funktionalität aufzubauen.
)

(event EventTick
  (params (DeltaSeconds :type Float%20%28single-precision%29))
  (|CallParentFunction DeltaSeconds) ; Dieser Knoten ist deaktiviert und wird nicht aufgerufen.\nZiehe die Pins ab, um die Funktionalität aufzubauen.
)

(fn ConstructionScript
  (|CallParentFunction))