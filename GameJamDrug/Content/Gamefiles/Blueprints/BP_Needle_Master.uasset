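; BP_Needle_Master is the needle item logic that, on IA_Needle input, raises the player's SanityScore and triggers a timed level switch.
; The score increase is capped at the character's MaxInsanityScore.
; It then calls SwitchLevel on the test or regular level switcher, chosen by the game mode's CurrentlyTesting flag, with EffectDuration reduced by the character's NeedlePenaltyScore.
; Debug prints show the new score and unscaled duration.
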(event Input|EnhancedActionEvents|EnhancedInputActionIA_Needle
  (params (ActionValue :type Boolean) (ElapsedSeconds :type Float%20%28double-precision%29) (TriggeredSeconds :type Float%20%28double-precision%29) (InputAction :type Input%20Action%20Object%20Reference :default "/Game/Gamefiles/Input/Actions/IA_Needle.IA_Needle"))
  (CallFunction|NeedleInput))

(event EventBeginPlay
  (bind _returnvalue (Actor|GetActorOfClass "/Game/Gamefiles/Blueprints/BP_ThirdPersonGameMode.BP_ThirdPersonGameMode_C"))
  (Variables|Default|SetGameModeRef _returnvalue)
  (bind _asbp_third_person_character (Utilities|Casting|CastToBP_ThirdPersonCharacter (Game|GetPlayerCharacter 0)))
  (Variables|Default|SetAs%20BP%20Third%20Person%20Character _asbp_third_person_character))

(event Collision|EventActorBeginOverlap
  (params (OtherActor :type Actor%20Object%20Reference)))

(fn ConstructionScript)

(fn NeedleInput
  (bind _effectduration (Variables|Default|GetEffectDuration))
  (bind _as_bp_third_person_character (Variables|Default|GetAs%20BP%20Third%20Person%20Character))
  (bind _needlepenaltyscore (Variables|/Game/Gamefiles/Blueprints/BP_ThirdPersonCharacter.BP_ThirdPersonCharacter_C|GetNeedlePenaltyScore _as_bp_third_person_character))
  (bind _returnvalue (- 1.0 _needlepenaltyscore))
  (bind _returnvalue_2 (* _effectduration _returnvalue))
  (bind _asbp_third_person_character (Utilities|Casting|CastToBP_ThirdPersonCharacter (Game|GetPlayerCharacter 0)))
  (bind _output_get (Variables|/Game/Gamefiles/Blueprints/BP_ThirdPersonCharacter.BP_ThirdPersonCharacter_C|SetSanityScore _asbp_third_person_character (Math|Float|Min(Float) (+ (Variables|Default|GetSanityIncrease) (Variables|/Game/Gamefiles/Blueprints/BP_ThirdPersonCharacter.BP_ThirdPersonCharacter_C|GetSanityScore _asbp_third_person_character)) (Variables|/Game/Gamefiles/Blueprints/BP_ThirdPersonCharacter.BP_ThirdPersonCharacter_C|GetMaxInsanityScore _asbp_third_person_character))))
  (Development|PrintText (Utilities|Text|ToText(Float) _output_get "HalfToEven"))
  (if (Variables|/Game/Gamefiles/Blueprints/BP_ThirdPersonGameMode.BP_ThirdPersonGameMode_C|GetCurrentlyTesting? (Variables|Default|GetGameModeRef))
    (bind _returnvalue_3 (Actor|GetActorOfClass "/Game/Gamefiles/Blueprints/BP_Level_Switcher_for_Test.BP_Level_Switcher_for_Test_C"))
    (Utilities|IsValid _returnvalue_3
      (:Is%20Valid
        (Default|SwitchLevel _returnvalue_3 _returnvalue_2)))
    (else
      (bind _returnvalue_4 (Actor|GetActorOfClass "/Game/Gamefiles/Blueprints/BP_Level_Switcher.BP_Level_Switcher_C"))
      (Utilities|IsValid _returnvalue_4
        (:Is%20Valid
          (Default|SwitchLevel _returnvalue_4 _returnvalue_2)))))
  (Development|PrintText "Effect Duration: ")
  (Development|PrintText (Utilities|Text|ToText(Float) _effectduration "HalfToEven")))