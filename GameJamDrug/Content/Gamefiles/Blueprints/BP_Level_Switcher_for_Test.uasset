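; Test-only level switcher that swaps between dark and light world variants of the prototyping level as streamed level instances.
; On BeginPlay it flags the GameMode as testing, loads the dark world and teleports the player to PlayerStart_Dark.
; SwitchLevel enters the light world for a given duration, or returns to dark if already light or given zero.
; Swaps unload the other instance and update the character's IsInLightWorld.
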(event Custom|SwitchbackToWorld
  (params (Duration_in_Light_World :type Float%20%28double-precision%29))
  (Utilities|FlowControl|Delay Duration_in_Light_World)
  (CallFunction|LoadLevelDark))

(event Custom|Despawn%20Level
  (params (Level_To_Despawn :type Level%20Streaming%20Object%20Reference))
  (Utilities|IsValid Level_To_Despawn
    (:Is%20Valid
      (Class|LevelStreaming|SetIsRequestingUnloadandRemoval Level_To_Despawn true))))

(event EventBeginPlay
  (bind _returnvalue (Actor|GetActorOfClass "/Game/Gamefiles/Blueprints/BP_ThirdPersonGameMode.BP_ThirdPersonGameMode_C"))
  (Variables|/Game/Gamefiles/Blueprints/BP_ThirdPersonGameMode.BP_ThirdPersonGameMode_C|SetCurrentlyTesting? _returnvalue true)
  (CallFunction|SwitchLevel 0.0)
  (Utilities|FlowControl|Delay 0.2)
  (CallFunction|SetPlayertoSpawnLocationinLevelDark))

(event Collision|EventActorBeginOverlap
  (params (OtherActor :type Actor%20Object%20Reference)))

(event EventTick
  (params (DeltaSeconds :type Float%20%28single-precision%29)))

(fn ConstructionScript)

(fn SwitchLevel
  (params (Duration_in_light_Word :type Float%20%28double-precision%29))
  (if (== Duration_in_light_Word 0.0)
    (CallFunction|LoadLevelDark :!label _label)
    (elif (Variables|Default|GetLight_World)
      (goto _label)
      (else
        (CallFunction|LoadLevelLight)
        (CallFunction|SwitchbacktoWorld Duration_in_light_Word)))))

(fn LoadLevelDark
  (bind _level_light (Variables|Default|GetLevel_Light))
  (bind _returnvalue (Class|LevelStreamingDynamic|LoadLevelInstancebySoftObjectPtr "/Game/Gamefiles/Maps/Prototyping_Level.Prototyping_Level" "0, 0, 0" "0, 0, 0" "" 0 false))
  (Variables|Default|SetLevel_Dark _returnvalue)
  (Utilities|IsValid _level_light
    (:Is%20Valid
      (if (Variables|Default|GetLight_World)
        (CallFunction|DespawnLevel _level_light)
        (Variables|Default|SetLight_World false)
        (bind _asbp_third_person_character (Utilities|Casting|CastToBP_ThirdPersonCharacter (Game|GetPlayerCharacter 0)))
        (Variables|/Game/Gamefiles/Blueprints/BP_ThirdPersonCharacter.BP_ThirdPersonCharacter_C|SetIs_in_Light_World _asbp_third_person_character (Variables|Default|GetLight_World))))))

(fn LoadLevelLight
  (bind _returnvalue (Class|LevelStreamingDynamic|LoadLevelInstancebySoftObjectPtr "/Game/Gamefiles/Maps/Prototyping_Level_light.Prototyping_Level_light" "0, 0, 0" "0, 0, 0" "" 0 false))
  (Variables|Default|SetLevel_Light _returnvalue)
  (CallFunction|DespawnLevel (Variables|Default|GetLevel_Dark))
  (bind _output_get (Variables|Default|SetLight_World true))
  (bind _asbp_third_person_character (Utilities|Casting|CastToBP_ThirdPersonCharacter (Game|GetPlayerCharacter 0)))
  (Variables|/Game/Gamefiles/Blueprints/BP_ThirdPersonCharacter.BP_ThirdPersonCharacter_C|SetIs_in_Light_World _asbp_third_person_character _output_get))

(fn SetPlayertoSpawnLocationinLevelDark
  (bind _outactors (Actor|GetAllActorsOfClass "/Script/Engine.PlayerStart"))
  (for _array_element _outactors
    (if (Utilities|Enum|Equal(Enum) (Utilities|GetDisplayName _array_element) "PlayerStart_Dark")
      (bind _output_get (Variables|Default|SetPlayerPositionInDark _array_element))))
  (Utilities|IsValid _output_get
    (:Is%20Valid
      (bind _asbp_third_person_character (Utilities|Casting|CastToBP_ThirdPersonCharacter (Game|GetPlayerCharacter 0)))
      (Transformation|SetActorTransform _asbp_third_person_character (Transformation|GetActorTransform _output_get) false true))))