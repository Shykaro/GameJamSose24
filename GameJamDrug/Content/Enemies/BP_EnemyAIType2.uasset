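; Enemy AI character that chases the player on sight via PawnSensing and AIMoveTo, attacking on arrival with a montage-length cooldown.
; Tick grows the capsule and resets HP to a scaled base value as the player's InsanityScore drops below max, discarding damage taken whenever the score changes.
; Attack damage instead rises with InsanityScore.
; EnemyTakeDmg subtracts HP; Tick handles death and destruction, while both montage calls have no animation assigned.
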(event OnSeePawn(PawnSensing)
  (params (Pawn :type Pawn%20Object%20Reference))
  (Variables|Default|SetEnemyIsSeeingPlayer true)
  (CallFunction|FollowPlayer))

(event Custom|Follow%20Player
  (bind _playercharacter_ref (Variables|Default|GetPlayerCharacter%20REF))
  (if (Variables|Default|GetEnemyIsSeeingPlayer)
    (AI|AIMoveTo self "0, 0, 0" (Game|GetPlayerCharacter 0) 5.0 false
      (:OnSuccess
        (if (Variables|Default|GetEnemyCanAttack)
          (Default|TakeDamage _playercharacter_ref (* (Variables|Default|GetEnemyDamage) (+ (/ (Variables|/Game/Gamefiles/Blueprints/BP_ThirdPersonCharacter.BP_ThirdPersonCharacter_C|GetInsanityScore _playercharacter_ref) (Variables|/Game/Gamefiles/Blueprints/BP_ThirdPersonCharacter.BP_ThirdPersonCharacter_C|GetMaxInsanityScore _playercharacter_ref)) 1.0)))
          (Variables|Default|SetEnemyCanAttack false)
          ;[0 0 0] Hier fehlt ne Animation
          (bind _returnvalue (Animation|PlayAnimMontage 0 1.0 "None"))
          (Utilities|FlowControl|Delay _returnvalue)
          (Variables|Default|SetEnemyCanAttack true))))))

(event EventBeginPlay
  ;[0 0 0] Set reference for player
  (bind _asbp_third_person_character (Utilities|Casting|CastToBP_ThirdPersonCharacter (Game|GetPlayerCharacter 0)))
  (Variables|Default|SetPlayerCharacter%20REF _asbp_third_person_character)
  (Variables|Default|SetPreviousInsanityScore (Variables|/Game/Gamefiles/Blueprints/BP_ThirdPersonCharacter.BP_ThirdPersonCharacter_C|GetInsanityScore (Variables|Default|GetPlayerCharacter%20REF))))

(event EventTick
  (params (DeltaSeconds :type Float%20%28single-precision%29))
  (bind _playercharacter_ref (Variables|Default|GetPlayerCharacter%20REF))
  (bind _playercharacter_ref_2 (Variables|Default|GetPlayerCharacter%20REF))
  (bind _insanityscore (Variables|/Game/Gamefiles/Blueprints/BP_ThirdPersonCharacter.BP_ThirdPersonCharacter_C|GetInsanityScore _playercharacter_ref_2))
  (bind _insanityscore_2 (Variables|/Game/Gamefiles/Blueprints/BP_ThirdPersonCharacter.BP_ThirdPersonCharacter_C|GetInsanityScore _playercharacter_ref))
  (bind _maxinsanityscore (Variables|/Game/Gamefiles/Blueprints/BP_ThirdPersonCharacter.BP_ThirdPersonCharacter_C|GetMaxInsanityScore _playercharacter_ref_2))
  (bind _maxinsanityscore_2 (Variables|/Game/Gamefiles/Blueprints/BP_ThirdPersonCharacter.BP_ThirdPersonCharacter_C|GetMaxInsanityScore _playercharacter_ref))
  (bind _returnvalue (- _maxinsanityscore_2 _insanityscore_2))
  (bind _returnvalue_2 (/ _returnvalue _maxinsanityscore_2))
  (bind _returnvalue_3 (+ _returnvalue_2 1.0))
  (Utilities|FlowControl|Sequence
    (:then_0
      ;[0 0 0] Enemy death
      (if (<= (Variables|Default|GetEnemyHP) 0.0)
        (Components|Movement|StopMovementImmediately (Variables|Character|GetCharacterMovement))
        (bind _returnvalue_4 (Animation|PlayAnimMontage 0 1.0 "None"))
        (Variables|Default|SetEnemyIsDead true)
        (Utilities|FlowControl|Delay _returnvalue_4)
        (Actor|DestroyActor)))
    (:then_1
      ;[0 0 0] Skaliert Gegnergröße
      (if (not (<= _returnvalue_3 1.0))
        (bind _output_get (Variables|Default|SetEnemyScaleFactor _returnvalue_3))
        (Transformation|SetWorldScale3D (Variables|Collision|GetCapsuleComponent) (Math|Conversions|ToVector(Float) _output_get))))
    (:then_2
      ;[0 0 0] HP Scaling
      (if (!= (Variables|/Game/Gamefiles/Blueprints/BP_ThirdPersonCharacter.BP_ThirdPersonCharacter_C|GetInsanityScore (Variables|Default|GetPlayerCharacter%20REF)) (Variables|Default|GetPreviousInsanityScore))
        (Variables|Default|SetEnemyHP (* (+ (/ (- _maxinsanityscore _insanityscore) _maxinsanityscore) 1.0) (Variables|Default|GetEnemyBaseHP)))
        (Variables|Default|SetPreviousInsanityScore _insanityscore)))))

(fn ConstructionScript)

(fn EnemyTakeDmg
  (params (PlayerDamage :type Float%20%28double-precision%29))
  (Variables|Default|SetEnemyHP (- (Variables|Default|GetEnemyHP) PlayerDamage)))