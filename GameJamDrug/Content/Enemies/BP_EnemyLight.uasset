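; BP_EnemyLight is an enemy that flees the player when the player is in the light world.
; On BeginPlay it caches the player character and insanity score, and starts AvoidPlayer if that world is active.
; AvoidPlayer moves to a random reachable point around a spot 500 units directly away from the player, re-calling itself on success or failure.
; EnemyTakeDmg only subtracts HP; a delayed FollowPlayer call is left unconnected.
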(event Custom|AvoidPlayer
  (bind _returnvalue (Transformation|GetActorLocation))
  (bind _playercharacter_ref (Variables|Default|GetPlayerCharacter%20REF))
  (bind _returnvalue_2 (Transformation|GetActorLocation _playercharacter_ref))
  (bind _returnvalue_3 (Math|Rotator|FindLookatRotation _returnvalue _returnvalue_2))
  (bind _returnvalue_4 (Math|Vector|GetForwardVector _returnvalue_3))
  (bind _returnvalue_5 (* _returnvalue_4 -5e+02))
  (bind _returnvalue_6 (+ _returnvalue _returnvalue_5))
  (bind (_x _y) (Math|Vector|BreakVector _returnvalue_6))
  (AI|AIMoveTo self (.RandomLocation (AI|Navigation|GetRandomReachablePointinRadius (Math|Vector|MakeVector _x _y (.Z (Math|Vector|BreakVector _returnvalue))) 5e+02 0 0)) 0 5.0 false
    (:OnSuccess
      _)
    (:OnFail
      _))
  (CallFunction|AvoidPlayer))

(event EventBeginPlay
  (Utilities|FlowControl|Sequence
    (:then_0
      ;[0 0 0] Set reference for player
      (bind _asbp_third_person_character (Utilities|Casting|CastToBP_ThirdPersonCharacter (Game|GetPlayerCharacter 0)))
      (Variables|Default|SetPlayerCharacter%20REF _asbp_third_person_character)
      (Variables|Default|SetPreviousInsanityScore (Variables|/Game/Gamefiles/Blueprints/BP_ThirdPersonCharacter.BP_ThirdPersonCharacter_C|GetInsanityScore (Variables|Default|GetPlayerCharacter%20REF))))
    (:then_4
      (if (Variables|/Game/Gamefiles/Blueprints/BP_ThirdPersonCharacter.BP_ThirdPersonCharacter_C|GetIs_in_Light_World (Variables|Default|GetPlayerCharacter%20REF))
        (CallFunction|AvoidPlayer)))))

(fn ConstructionScript)

(fn EnemyTakeDmg
  (params (PlayerDamage :type Float%20%28double-precision%29))
  (Variables|Default|SetEnemyHP (- (Variables|Default|GetEnemyHP) PlayerDamage)))