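; BP_EnemySpawner is a spawner actor that keeps producing enemies when the player starts outside the light world.
; At BeginPlay it finds the BP_ThirdPersonCharacter and, if IsInLightWorld is false, starts a looping one-second timer; the state is never rechecked.
; Each tick of that timer spawns BP_EnemyAI, or less often BP_EnemyAIType2, at random reachable navmesh X/Y within SpawnRadius and a fixed height, printing a debug message.
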(event Custom|SpawnEnemy
  (bind _returnvalue (Transformation|GetActorLocation))
  (bind _spawnradius (Variables|Default|GetSpawnRadius))
  (bind _randomlocation (AI|Navigation|GetRandomReachablePointinRadius _returnvalue _spawnradius 0 0))
  (if (>= (Math|Random|RandomFloatinRange 0.0 1.0) 0.8)
    (Game|SpawnActorfromClass "/Game/Enemies/BP_EnemyAIType2.BP_EnemyAIType2_C" (Math|Transform|MakeTransform (Math|Vector|MakeVector (.x _randomlocation) (.y _randomlocation) 1e+02) "0, 0, 0" "1.000000,1.000000,1.000000") "Undefined" "MultiplyWithRoot" 0 0)
    (Development|PrintString "anderer Atze spawned")
    (else
      (Game|SpawnActorfromClass "/Game/Enemies/BP_EnemyAI.BP_EnemyAI_C" (Math|Transform|MakeTransform (Math|Vector|MakeVector (.x _randomlocation) (.y _randomlocation) 1e+02) "0, 0, 0" "1.000000,1.000000,1.000000") "Undefined" "MultiplyWithRoot" 0 0)
      (Development|PrintString "Atze spawned"))))

(event EventBeginPlay
  (Utilities|FlowControl|Sequence
    (:then_0
      (bind _returnvalue (Actor|GetActorOfClass "/Game/Gamefiles/Blueprints/BP_ThirdPersonCharacter.BP_ThirdPersonCharacter_C"))
      (Variables|Default|SetAs%20BP%20Third%20Person%20Char _returnvalue))
    (:then_1
      (if (not (Variables|/Game/Gamefiles/Blueprints/BP_ThirdPersonCharacter.BP_ThirdPersonCharacter_C|GetIs_in_Light_World (Variables|Default|GetAs%20BP%20Third%20Person%20Char)))
        (Utilities|Time|SetTimerbyEvent (delegate Custom|SpawnEnemy) 1.0 true)))))

(fn ConstructionScript)