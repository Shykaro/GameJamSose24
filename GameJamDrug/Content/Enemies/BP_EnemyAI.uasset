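; Enemy AI character that voices and chases the player when seen or heard, dealing sanity-scaled melee damage with a montage-based cooldown.
; A looping timer raises HP as player sanity drops, while Tick grows its capsule likewise and handles a sinking death before destruction.
; In the Light World it slowly retreats to random reachable points away from the player, resuming pursuit after the needle effect's duration.
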(event OnSeePawn(PawnSensing)
  (params (Pawn :type Pawn%20Object%20Reference))
  (bind _capsulecomponent (Variables|Collision|GetCapsuleComponent))
  ;[0.1094 0.1094 0.1094] On See Pawn
  (switch int (Math|Random|RandomIntegerinRange 0 2)
    (:0
      (Audio|SpawnSoundAttached "/Game/Gamefiles/Sounds/EnemyVoice1.EnemyVoice1" _capsulecomponent "None" "0, 0, 0" "0, 0, 0" "KeepRelativeOffset" false 1.0 1.0 0.0 0 0))
    (:1
      (Audio|SpawnSoundAttached "/Game/Gamefiles/Sounds/EnemyVoice2.EnemyVoice2" _capsulecomponent "None" "0, 0, 0" "0, 0, 0" "KeepRelativeOffset" false 1.0 1.0 0.0 0 0))
    (:2
      (Audio|SpawnSoundAttached "/Game/Gamefiles/Sounds/EnemyVoice3.EnemyVoice3" _capsulecomponent "None" "0, 0, 0" "0, 0, 0" "KeepRelativeOffset" false 1.0 1.0 0.0 0 0)))
  (Variables|Default|SetEnemyIsSeeingPlayer true)
  (if (Variables|/Game/Gamefiles/Blueprints/BP_ThirdPersonCharacter.BP_ThirdPersonCharacter_C|GetIs_in_Light_World (Variables|Default|GetPlayerCharacter%20REF))
    (CallFunction|AvoidPlayer)
    (else
      (CallFunction|FollowPlayer))))

(event OnHearNoise(PawnSensing)
  (params (Instigator :type Pawn%20Object%20Reference) (Location :type Vector%20%28by%20ref%29 :default "0, 0, 0") (Volume :type Float%20%28single-precision%29))
  (bind _capsulecomponent (Variables|Collision|GetCapsuleComponent))
  ;[0.1094 0.1094 0.1094] On See Pawn
  (switch int (Math|Random|RandomIntegerinRange 0 2)
    (:0
      (Audio|SpawnSoundAttached "/Game/Gamefiles/Sounds/EnemyVoice1.EnemyVoice1" _capsulecomponent "None" "0, 0, 0" "0, 0, 0" "KeepRelativeOffset" false 1.0 1.0 0.0 0 0))
    (:1
      (Audio|SpawnSoundAttached "/Game/Gamefiles/Sounds/EnemyVoice2.EnemyVoice2" _capsulecomponent "None" "0, 0, 0" "0, 0, 0" "KeepRelativeOffset" false 1.0 1.0 0.0 0 0))
    (:2
      (Audio|SpawnSoundAttached "/Game/Gamefiles/Sounds/EnemyVoice3.EnemyVoice3" _capsulecomponent "None" "0, 0, 0" "0, 0, 0" "KeepRelativeOffset" false 1.0 1.0 0.0 0 0)))
  (Variables|Default|SetEnemyIsSeeingPlayer true)
  (if (Variables|/Game/Gamefiles/Blueprints/BP_ThirdPersonCharacter.BP_ThirdPersonCharacter_C|GetIs_in_Light_World (Variables|Default|GetPlayerCharacter%20REF))
    (CallFunction|AvoidPlayer)
    (else
      (CallFunction|FollowPlayer))))

(event Custom|Follow%20Player
  (bind _returnvalue (Game|GetPlayerCharacter 0))
  (bind _playercharacter_ref (Variables|Default|GetPlayerCharacter%20REF))
  ;[0.1146 0.1146 0.1146] Follow Player
  (if (Variables|Default|GetEnemyIsSeeingPlayer) :!label _label
    (Utilities|IsValid _returnvalue
      (:Is%20Valid
        (AI|AIMoveTo self "0, 0, 0" _returnvalue 5.0 false
          (:OnSuccess
            (if (Variables|Default|GetEnemyCanAttack)
              (Default|TakeDamage _playercharacter_ref (* (Variables|Default|GetEnemyDamage) (+ (/ (Variables|/Game/Gamefiles/Blueprints/BP_ThirdPersonCharacter.BP_ThirdPersonCharacter_C|GetSanityScore _playercharacter_ref) (Variables|/Game/Gamefiles/Blueprints/BP_ThirdPersonCharacter.BP_ThirdPersonCharacter_C|GetMaxInsanityScore _playercharacter_ref)) 1.0)))
              (Variables|Default|SetEnemyCanAttack false)
              (bind _returnvalue_2 (Animation|PlayAnimMontage "/Game/Enemies/Locomotion/EnemyAttkMon.EnemyAttkMon" 1.0 "None"))
              (Utilities|FlowControl|Delay _returnvalue_2)
              (Variables|Default|SetEnemyCanAttack true)))))
      (:Is%20Not%20Valid
        (Utilities|FlowControl|Delay 1.0)
        (goto _label)))))

(event Custom|AvoidPlayer
  (bind _returnvalue (Transformation|GetActorLocation))
  (bind _playercharacter_ref (Variables|Default|GetPlayerCharacter%20REF))
  (bind _returnvalue_2 (Transformation|GetActorLocation _playercharacter_ref))
  (bind _returnvalue_3 (Math|Rotator|FindLookatRotation _returnvalue _returnvalue_2))
  (bind _returnvalue_4 (Math|Vector|GetForwardVector _returnvalue_3))
  (bind _returnvalue_5 (* _returnvalue_4 -5e+02))
  (bind _returnvalue_6 (+ _returnvalue _returnvalue_5))
  (bind (_x _y) (Math|Vector|BreakVector _returnvalue_6))
  ;[0.1094 0.1094 0.1094] Avoid Player
  (Variables|/Script/Engine.CharacterMovementComponent|SetMaxWalkSpeed (Variables|Character|GetCharacterMovement) 1e+02)
  (AI|AIMoveTo self (.RandomLocation (AI|Navigation|GetRandomReachablePointinRadius (Math|Vector|MakeVector _x _y (.Z (Math|Vector|BreakVector _returnvalue))) 5e+02 0 0)) 0 5.0 false
    (:OnSuccess
      _)
    (:OnFail
      _))
  (CallFunction|AvoidPlayer))

(event Custom|ScaleEnemies
  (bind _playercharacter_ref (Variables|Default|GetPlayerCharacter%20REF))
  (bind _maxinsanityscore (Variables|/Game/Gamefiles/Blueprints/BP_ThirdPersonCharacter.BP_ThirdPersonCharacter_C|GetMaxInsanityScore _playercharacter_ref))
  ;[0.08854 0.08854 0.08854] Begin Play
  ;;[0 0 0] HP Scaling
  (bind _output_get (Variables|Default|SetEnemyHPAtLastScale (Variables|Default|GetCurrentMaxHP)))
  (bind _output_get_2 (Variables|Default|SetCurrentMaxHP (* (+ (/ (- _maxinsanityscore (Variables|/Game/Gamefiles/Blueprints/BP_ThirdPersonCharacter.BP_ThirdPersonCharacter_C|GetSanityScore _playercharacter_ref)) _maxinsanityscore) 1.0) (Variables|Default|GetEnemyBaseHP))))
  (bind _output_get_3 (Variables|Default|SetCurrentEnemyHP (+ (Variables|Default|GetCurrentEnemyHP) (- _output_get_2 _output_get)))))

(event EventBeginPlay
  ;[0.08854 0.08854 0.08854] Begin Play
  (Utilities|FlowControl|Sequence
    (:then_0
      (bind _asbp_third_person_character (Utilities|Casting|CastToBP_ThirdPersonCharacter (Game|GetPlayerCharacter 0)))
      (Variables|Default|SetPlayerCharacter%20REF _asbp_third_person_character)
      (Variables|Default|SetPreviousInsanityScore (Variables|/Game/Gamefiles/Blueprints/BP_ThirdPersonCharacter.BP_ThirdPersonCharacter_C|GetSanityScore (Variables|Default|GetPlayerCharacter%20REF)))
      (Variables|Default|SetCurrentMaxHP (Variables|Default|GetEnemyBaseHP))
      (Utilities|Time|SetTimerbyEvent (delegate Custom|ScaleEnemies) 1.0 true))))

(event EventTick
  (params (DeltaSeconds :type Float%20%28single-precision%29))
  (bind _returnvalue (Transformation|GetActorTransform))
  (bind _playercharacter_ref (Variables|Default|GetPlayerCharacter%20REF))
  (bind _playercharacter_ref_2 (Variables|Default|GetPlayerCharacter%20REF))
  (bind _sanityscore (Variables|/Game/Gamefiles/Blueprints/BP_ThirdPersonCharacter.BP_ThirdPersonCharacter_C|GetSanityScore _playercharacter_ref))
  (bind _maxinsanityscore (Variables|/Game/Gamefiles/Blueprints/BP_ThirdPersonCharacter.BP_ThirdPersonCharacter_C|GetMaxInsanityScore _playercharacter_ref))
  (Utilities|FlowControl|Sequence
    (:then_0
      ;[0 0 0] Enemy death
      (if (<= (Variables|Default|GetCurrentEnemyHP) 0.0)
        (Components|Movement|StopMovementImmediately (Variables|Character|GetCharacterMovement))
        (bind _z_translation1 (Timeline|DeathAnimTimeline Play)
          (:Update
            (Transformation|SetActorTransform (Math|Transform|MakeTransform (Math|Vector|MakeVector 0.0 0.0 (Math|Float|Lerp (.z (.location _returnvalue)) (- (.z (.location _returnvalue)) 2e+01) _z_translation1)) "0, 0, 0" "1.000000,1.000000,1.000000")))
          (:Finished
            (Audio|PlaySoundatLocation "/Game/Gamefiles/Sounds/death.death" (.location (Transformation|GetActorTransform)) "0, 0, 0" 1.0 1.0 0.0 0 0 0 0)
            (Variables|Default|SetEnemyIsDead true)
            (Actor|DestroyActor)))))
    (:then_1
      ;[0 0 0] Skaliert Gegnergröße
      (if (not (>= _sanityscore _maxinsanityscore))
        (bind _output_get (Variables|Default|SetEnemyScaleFactor (+ (/ (- _maxinsanityscore _sanityscore) _maxinsanityscore) 1.0)))
        (Transformation|SetWorldScale3D (Variables|Collision|GetCapsuleComponent) (Math|Conversions|ToVector(Float) _output_get))))
    (:then_2
      ;[0.09375 0.09375 0.09375] AvoidPlayer if in Lightworld
      (if (Variables|/Game/Gamefiles/Blueprints/BP_ThirdPersonCharacter.BP_ThirdPersonCharacter_C|GetIs_in_Light_World _playercharacter_ref_2)
        (CallFunction|AvoidPlayer)
        (Utilities|FlowControl|Delay (Variables|/Game/Gamefiles/Blueprints/BP_Needle_Master.BP_Needle_Master_C|GetEffectDuration (Variables|/Game/Gamefiles/Blueprints/BP_ThirdPersonCharacter.BP_ThirdPersonCharacter_C|GetNeedleReference _playercharacter_ref_2)))
        (CallFunction|FollowPlayer)))))

(fn ConstructionScript)

(fn EnemyTakeDmg
  (params (PlayerDamage :type Float%20%28double-precision%29))
  (Variables|Default|SetCurrentEnemyHP (- (Variables|Default|GetCurrentEnemyHP) PlayerDamage)))